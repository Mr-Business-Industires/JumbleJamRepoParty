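; Radio Blueprint with a function that plays a random noise from a sound array as non-spatial 2D audio at a randomized pitch.
; PlayRandomRadioNoise picks the index up to the array length inclusive, so it can land one past the last element.
; The IsPlayingAudio-guarded call to it is disconnected from any event, and BeginPlay and Tick are empty, so nothing in this Blueprint triggers playback.
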(event `self.ReceiveBeginPlay`)

(event `self.ReceiveTick`
  (params (DeltaSeconds :type "Float (single-precision)")))

(fn `Play Random Radio Noise`
  (`GameplayStatics.PlaySound2D` (`|GetArrayItem` (`self.Radio Array`) (`KismetMathLibrary.RandomIntegerInRange` 0 (`KismetArrayLibrary.Array_Length` (`self.Radio Array`)))) 1.0 (`KismetMathLibrary.RandomFloatInRange` 0.5 2.5) 0.0 null null))

(fn `UserConstructionScript`)